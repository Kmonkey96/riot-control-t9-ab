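; Game state Blueprint for an RTS that tracks a match countdown and a capped score.
; Each tick, while the maximum timer is at least one second, it subtracts server world time from that maximum and splits the remainder into minutes and seconds.
; The AddScore event increments the score by one until it reaches the maximum score.
; Nothing here handles the timer reaching zero or the score hitting its cap.
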(event Custom|AddScore
  (bind _score (Variables|Score|GetScore))
  (if (< _score (Variables|Score|GetMaxScore))
    (Math|Integer|IncrementInt _score)))

(event EventBeginPlay)

(event EventTick
  (params (DeltaSeconds :type Float%20%28single-precision%29))
  (bind _returnvalue (GameState|GetServerWorldTimeSeconds))
  (bind _gametimermax (Variables|HUD|GetGameTimerMax))
  (bind _returnvalue_2 (- _gametimermax _returnvalue))
  (if (not (< (Variables|HUD|GetGameTimerMax) 1.0))
    (Variables|HUD|SetGameCurrentTimer _returnvalue_2)
    (Variables|HUD|SetSeconds (Math|Float|Truncate (Math|Float|%(Float) _returnvalue_2 6e+01)))
    (Variables|HUD|SetMinutes (Math|Float|Floor (/ _returnvalue_2 6e+01)))))

(fn ConstructionScript)