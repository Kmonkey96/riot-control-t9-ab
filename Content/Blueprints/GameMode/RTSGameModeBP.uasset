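; RTS game mode that detects the running platform at BeginPlay and sets up a debug HUD to match.
; A chain of platform-name comparisons stores the result in a CurrentPlatform enum.
; It then creates a collapsed DebugHUD widget labeled with that platform.
; An enum comparison reveals the desktop debug box for the zero-valued platform entry and the mobile box for all others.
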(event EventBeginPlay
  (Utilities|FlowControl|Sequence
    (:then_0
      (bind _returnvalue (Game|GetPlatformName))
      (if (Utilities|Enum|Equal(Enum) _returnvalue "Windows")
        (Variables|Default|SetCurrentPlatform "NewEnumerator0")
        (elif (Utilities|Enum|Equal(Enum) _returnvalue "Linux")
          (Variables|Default|SetCurrentPlatform "NewEnumerator5")
          (elif (Utilities|Enum|Equal(Enum) _returnvalue "Mac")
            (Variables|Default|SetCurrentPlatform "NewEnumerator4")
            (elif (Utilities|Enum|Equal(Enum) _returnvalue "HTML5")
              (Variables|Default|SetCurrentPlatform "NewEnumerator3")
              (elif (Utilities|Enum|Equal(Enum) _returnvalue "Android")
                (Variables|Default|SetCurrentPlatform "NewEnumerator1")
                (elif (Utilities|Enum|Equal(Enum) _returnvalue "IOS")
                  (Variables|Default|SetCurrentPlatform "NewEnumerator2")
                  (elif (Utilities|Enum|Equal(Enum) _returnvalue "PS4")
                    (Variables|Default|SetCurrentPlatform "NewEnumerator6")
                    (elif (Utilities|Enum|Equal(Enum) _returnvalue "XboxOne")
                      (Variables|Default|SetCurrentPlatform "NewEnumerator7")
                      (elif (Utilities|Enum|Equal(Enum) _returnvalue "Unknown")
                        (Variables|Default|SetCurrentPlatform "NewEnumerator8")))))))))))
    (:then_1
      (bind _returnvalue_2 (UserInterface|CreateWidget "/Game/Blueprints/GUI/HUD/Debug/DebugHUD.DebugHUD_C" (Game|GetPlayerController 0) (Utilities|Text|ToText(String) (Utilities|String|EnumtoString (Variables|Default|GetCurrentPlatform)))))
      (Variables|Default|SetDebugHUDRef _returnvalue_2)
      (UserInterface|Viewport|AddtoViewport _returnvalue_2 0)
      (Widget|SetVisibility _returnvalue_2 "Collapsed"))
    (:then_2
      (if (<= (Variables|Default|GetCurrentPlatform) 0)
        (Widget|SetVisibility (Variables|/Game/Blueprints/GUI/HUD/Debug/DebugHUD.DebugHUD_C|GetDesktopDebug_VertBox (Variables|Default|GetDebugHUDRef)) "SelfHitTestInvisible")
        (else
          (Widget|SetVisibility (Variables|/Game/Blueprints/GUI/HUD/Debug/DebugHUD.DebugHUD_C|GetMobileDebug_VertBox (Variables|Default|GetDebugHUDRef)) "SelfHitTestInvisible"))))))

(fn ConstructionScript)